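; DroneBullet is a homing projectile actor that destroys the Target actor it is assigned.
; Each Tick moves it toward the target's current root location at constant speed with VInterpTo Constant, without sweeping for collision.
; A distance check stands in for hit detection, destroying both target and bullet once they nearly meet.
; The bullet also destroys itself whenever its target is no longer valid.
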(event EventTick
  (params (DeltaSeconds :type Float%20%28single-precision%29))
  (bind _defaultsceneroot (Variables|Default|GetDefaultSceneRoot))
  (bind _target (Variables|Default|GetTarget))
  (bind _returnvalue (Transformation|GetWorldLocation _defaultsceneroot))
  (bind _rootcomponent (Variables|/Script/Engine.Actor|GetRootComponent _target))
  (bind _returnvalue_2 (Transformation|GetWorldLocation _rootcomponent))
  (Utilities|IsValid (Variables|Default|GetTarget)
    (:Is%20Valid
      (if (<= (Math|Vector|VectorLength (- _returnvalue _returnvalue_2)) 1e+01)
        (Actor|DestroyActor (Variables|Default|GetTarget))
        (Actor|DestroyActor)
        (else
          (Transformation|SetActorLocation (Math|Interpolation|VInterptoConstant _returnvalue _returnvalue_2 DeltaSeconds 1e+03) false false))))
    (:Is%20Not%20Valid
      (Actor|DestroyActor))))

(fn ConstructionScript)