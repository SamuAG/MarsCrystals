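; Enemigo is an enemy that chases the player pawn every tick using SimpleMoveToActor.
; When its Box overlaps the third-person character, it subtracts 10 from Health stored on the game mode, opens DesertLevel if that reaches zero or below, and updates the character's HUD.
; It then destroys itself, and its Destroyed event spawns an Explosion at the capsule's transform.
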(event OnComponentBeginOverlap(Box)
  (params (OverlappedComponent :type Primitive%20Component%20Object%20Reference) (OtherActor :type Actor%20Object%20Reference) (OtherComp :type Primitive%20Component%20Object%20Reference) (OtherBodyIndex :type Integer) (bFromSweep :type Boolean) (SweepResult :type Hit%20Result%20Structure%20%28by%20ref%29))
  (bind _asbp_third_person_character (Utilities|Casting|CastToBP_ThirdPersonCharacter OtherActor))
  (bind _asbp_third_person_game_mode (Utilities|Casting|CastToBP_ThirdPersonGameMode (Game|GetGameMode)))
  (bind _output_get (Variables|/Game/ThirdPerson/Blueprints/BP_ThirdPersonGameMode.BP_ThirdPersonGameMode_C|SetHealth _asbp_third_person_game_mode (- (Variables|/Game/ThirdPerson/Blueprints/BP_ThirdPersonGameMode.BP_ThirdPersonGameMode_C|GetHealth _asbp_third_person_game_mode) 10)))
  (if (<= _output_get 0)
    (Game|OpenLevel(byName) "DesertLevel"))
  (Default|UpdateHealth (Variables|/Game/ThirdPerson/Blueprints/BP_ThirdPersonCharacter.BP_ThirdPersonCharacter_C|GetRealHUD _asbp_third_person_character) (Utilities|Text|ToText(Integer) _output_get))
  (Actor|DestroyActor))

(event EventDestroyed
  (Game|SpawnActorfromClass "/Game/StarterContent/Particles/Explosion.Explosion_C" (Transformation|GetWorldTransform (Variables|Collision|GetCapsuleComponent)) "AlwaysSpawn" "MultiplyWithRoot" 0 0))

(event EventTick
  (params (DeltaSeconds :type Float%20%28single-precision%29))
  (AI|Navigation|SimpleMovetoActor (Pawn|GetController) (Game|Player|GetPlayerPawn 0)))

(fn ConstructionScript)