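; Companion drone that trails the player's DronePosition on the third-person character or offroad car, with a cosine bobbing offset.
; Each Tick, it eases location and rotation toward that anchor using Lerps weighted to its current transform.
; In the character's top-down mode, it scans all Enemigo actors for the nearest, though the comparison clears closer candidates rather than assigning them.
; A target within range makes it turn and fire targeted DroneBullets on a Delay-based cooldown.
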(event EventTick
  (params (DeltaSeconds :type Float%20%28single-precision%29))
  (bind _returnvalue (Game|Player|GetPlayerPawn 0))
  (bind _returnvalue_2 (Transformation|GetActorLocation))
  (bind _defaultsceneroot (Variables|Default|GetDefaultSceneRoot))
  (bind _defaultsceneroot_2 (Variables|Default|GetDefaultSceneRoot))
  (bind _defaultsceneroot_3 (Variables|Default|GetDefaultSceneRoot))
  ;[1 1 1] ThirdPerson
  (bind _asbp_third_person_character (Utilities|Casting|CastToBP_ThirdPersonCharacter _returnvalue)
    (:then
      (if (Variables|/Game/ThirdPerson/Blueprints/BP_ThirdPersonCharacter.BP_ThirdPersonCharacter_C|GetTopDownMode _asbp_third_person_character)
        ;[1 1 1] Loojk to nearest enemy
        (bind _outactors (Actor|GetAllActorsOfClass "/Game/Blueprints/Enemigo.Enemigo_C"))
        (if (Utilities|Array|IsEmpty _outactors)
          (Transformation|SetActorTransform (Math|Transform|MakeTransform (Math|Vector|Lerp(Vector) (.location (Transformation|GetWorldTransform (Variables|/Game/ThirdPerson/Blueprints/BP_ThirdPersonCharacter.BP_ThirdPersonCharacter_C|GetDronePosition _asbp_third_person_character))) (Transformation|GetWorldLocation _defaultsceneroot_3) 0.92) (Math|Rotator|Lerp(Rotator) (Transformation|GetWorldRotation _defaultsceneroot_3) (Math|Rotator|MakeRotator (.roll (.rotation (Transformation|GetWorldTransform (Variables|/Game/ThirdPerson/Blueprints/BP_ThirdPersonCharacter.BP_ThirdPersonCharacter_C|GetDronePosition _asbp_third_person_character)))) (.pitch (.rotation (Transformation|GetWorldTransform (Variables|/Game/ThirdPerson/Blueprints/BP_ThirdPersonCharacter.BP_ThirdPersonCharacter_C|GetDronePosition _asbp_third_person_character)))) (+ (.yaw (.rotation (Transformation|GetWorldTransform (Variables|/Game/ThirdPerson/Blueprints/BP_ThirdPersonCharacter.BP_ThirdPersonCharacter_C|GetDronePosition _asbp_third_person_character)))) -9e+01)) 0.99) "0.200000,0.200000,0.200000") true :!label _label)
          ;[1 1 1] Float effect
          (Transformation|AddRelativeLocation (Variables|Default|GetStaticMesh) (* (Math|Vector|MakeVector 0.0 0.0 (* (Math|Trig|Cos(Radians) (Actor|GetGameTimeSinceCreation)) 5e+01)) DeltaSeconds) false false :!label _label_2)
          (else
            (for _array_element _outactors
              (Utilities|IsValid 0
                (:Is%20Valid
                  (if (< (Math|Vector|VectorLength (- _returnvalue_2 (Transformation|GetWorldLocation (Variables|/Script/Engine.Actor|GetRootComponent _array_element)))) (Math|Vector|VectorLength (- _returnvalue_2 (Transformation|GetWorldLocation (Variables|/Script/Engine.Actor|GetRootComponent (Variables|Default|GetnearestEnemigo))))))
                    (Variables|Default|SetnearestEnemigo 0)))
                (:Is%20Not%20Valid
                  (Variables|Default|SetnearestEnemigo _array_element))))
            (if (< (Math|Vector|VectorLength (- (Transformation|GetActorLocation) (Transformation|GetWorldLocation (Variables|/Script/Engine.Actor|GetRootComponent (Variables|Default|GetnearestEnemigo))))) 6e+02)
              (Transformation|SetActorTransform (Math|Transform|MakeTransform (Math|Vector|Lerp(Vector) (.location (Transformation|GetWorldTransform (Variables|/Game/ThirdPerson/Blueprints/BP_ThirdPersonCharacter.BP_ThirdPersonCharacter_C|GetDronePosition _asbp_third_person_character))) (Transformation|GetWorldLocation _defaultsceneroot_2) 0.92) (Math|Rotator|Lerp(Rotator) (Transformation|GetWorldRotation _defaultsceneroot_2) (Math|Rotator|MakeRotator (.roll (Math|Rotator|FindLookatRotation (Transformation|GetActorLocation) (Transformation|GetActorLocation (Variables|Default|GetnearestEnemigo)))) 0.0 (+ (.yaw (Math|Rotator|FindLookatRotation (Transformation|GetActorLocation) (Transformation|GetActorLocation (Variables|Default|GetnearestEnemigo)))) -9e+01)) 0.99) "0.200000,0.200000,0.200000") true)
              (if (Variables|Default|GetCanShoot)
                (Variables|Default|SetCanShoot false)
                (bind _returnvalue_3 (Game|SpawnActorfromClass "/Game/Blueprints/DroneBullet.DroneBullet_C" (Transformation|GetWorldTransform (Variables|Default|GetDefaultSceneRoot)) "Undefined" "MultiplyWithRoot" 0 0))
                (bind _asdrone_bullet (Utilities|Casting|CastToDroneBullet _returnvalue_3))
                (Variables|/Game/Blueprints/DroneBullet.DroneBullet_C|SetTarget _asdrone_bullet (Variables|Default|GetnearestEnemigo))
                (Utilities|FlowControl|Delay 2.0)
                (Variables|Default|SetCanShoot true)
                (else
                  (goto _label_2)))
              (else
                (goto _label)))))
        (else
          (goto _label))))
    (:CastFailed
      ;[1 1 1] Car mode
      (bind _asoffroad_car_pawn (Utilities|Casting|CastToOffroadCar_Pawn _returnvalue))
      (Transformation|SetActorTransform (Math|Transform|MakeTransform (Math|Vector|Lerp(Vector) (.location (Transformation|GetWorldTransform (Variables|/Game/VehicleTemplate/Blueprints/OffroadCar/OffroadCar_Pawn.OffroadCar_Pawn_C|GetDronePosition _asoffroad_car_pawn))) (Transformation|GetWorldLocation _defaultsceneroot) 0.9) (Math|Rotator|Lerp(Rotator) (Transformation|GetWorldRotation _defaultsceneroot) (Math|Rotator|MakeRotator (.roll (.rotation (Transformation|GetWorldTransform (Variables|/Game/VehicleTemplate/Blueprints/OffroadCar/OffroadCar_Pawn.OffroadCar_Pawn_C|GetDronePosition _asoffroad_car_pawn)))) (.pitch (.rotation (Transformation|GetWorldTransform (Variables|/Game/VehicleTemplate/Blueprints/OffroadCar/OffroadCar_Pawn.OffroadCar_Pawn_C|GetDronePosition _asoffroad_car_pawn)))) (+ (.yaw (.rotation (Transformation|GetWorldTransform (Variables|/Game/VehicleTemplate/Blueprints/OffroadCar/OffroadCar_Pawn.OffroadCar_Pawn_C|GetDronePosition _asoffroad_car_pawn)))) -9e+01)) 0.99) "0.200000,0.200000,0.200000") true)
      (goto _label_2))))

(fn ConstructionScript)