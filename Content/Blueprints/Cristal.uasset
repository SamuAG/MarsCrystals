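; Collectible crystal that springs an enemy ambush when the player character touches it and counts toward winning the level.
; On BeginPlay it records how many crystals exist and applies its material to the cube.
; The first player overlap spawns enemies at spawn points offset from its location, increments the GameMode tally and updates the HUD.
; It shows the Win widget once the tally reaches the recorded total, then destroys itself.
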(event EventBeginPlay
  (bind _outactors (Actor|GetAllActorsOfClass "Cristal_C"))
  (Variables|Default|SetCristalNumber (Utilities|Array|Length _outactors))
  (Rendering|Material|SetMaterial (Variables|Default|GetCube) 0 (Variables|Default|GetMat)))

(event Collision|EventActorBeginOverlap
  (params (OtherActor :type Actor%20Object%20Reference))
  (bind _asbp_third_person_character (Utilities|Casting|CastToBP_ThirdPersonCharacter OtherActor))
  (if (not (Variables|Default|GetHasBeenEnabled))
    (Variables|Default|SetHasBeenEnabled true)
    (for _array_element (Variables|Default|GetSpawnPoints)
      (Game|SpawnActorfromClass (Variables|Default|GetEnemyBP) (Math|Transform|MakeTransform (+ (.location _array_element) (Transformation|GetWorldLocation (Variables|Default|GetDefaultSceneRoot))) (.rotation _array_element) "1.000000,1.000000,1.000000") "Undefined" "MultiplyWithRoot" 0 0))
    (bind _asbp_third_person_game_mode (Utilities|Casting|CastToBP_ThirdPersonGameMode (Game|GetGameMode))
      (:then
        (bind _result (Math|Integer|IncrementInt (Variables|/Game/ThirdPerson/Blueprints/BP_ThirdPersonGameMode.BP_ThirdPersonGameMode_C|GetCristals _asbp_third_person_game_mode))
          (:%20%20
            (Default|UpdateCristal (Variables|/Game/ThirdPerson/Blueprints/BP_ThirdPersonCharacter.BP_ThirdPersonCharacter_C|GetRealHUD _asbp_third_person_character) (Utilities|Text|ToText(Integer) _result))
            (if (>= _result (Variables|Default|GetCristalNumber))
              (bind _returnvalue (UserInterface|CreateWidget "/Game/UI/Win.Win_C"))
              (UserInterface|Viewport|AddtoViewport _returnvalue 0)))))
      (:CastFailed
        _))
    (Actor|DestroyActor)))

(fn ConstructionScript)